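; Player-controlled rolling ball Blueprint that moves by physics torque and can jump.
; The forwardbackward and leftright axis inputs drive one AddTorqueInRadians call on the Sphere, scaled by Ballspeed and applied as an acceleration change.
; Jump applies an upward velocity-change impulse of Jumpheight, gated by a DoOnce that resets after a short delay following button release rather than a ground check.
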(event `InputAxis|forwardbackward`
  (params (AxisValue :type "Float (single-precision)"))
  (bind _ballspeed (`self.ballspeed`))
  (`PrimitiveComponent.AddTorqueInRadians` (`self.Sphere`) (`KismetMathLibrary.MakeVector` (* (* (stale `InputAxis|leftright` AxisValue) _ballspeed) -1.0) (* AxisValue _ballspeed)) "None" true :!label _label))

(event `InputAxis|leftright`
  (params (AxisValue :type "Float (single-precision)"))
  (goto _label))

(event `InputAction|jump`
  (params (Key :type "Key Structure"))
  (:`Pressed`
    (`/Engine/EditorBlueprintResources/StandardMacros.DoOnce` false :!label _label_2
      (:`Completed`
        (`PrimitiveComponent.AddImpulse` (`self.Sphere`) (`KismetMathLibrary.MakeVector` 0.0 0.0 (`self.jumpheight`)) "None" true))))
  (:`Released`
    (`KismetSystemLibrary.Delay` 1.2)
    (goto _label_2 :!via `Reset`)))

(fn `UserConstructionScript`)